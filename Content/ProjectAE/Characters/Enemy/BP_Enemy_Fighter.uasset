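; Melee fighter enemy that extends its parent's attack flow and sets walk speed per movement state.
; Before the montage plays, it randomly picks a section from close or range attacks, favoring close ones when the player is within attack range.
; Close attacks box-trace forward; range attacks sphere-trace ahead, ignoring prior hits until cooldown reset, with JumpAttack adding a wider radius and ground decal.
; Player hits receive GAS damage through a SetByCaller effect.
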(fn `ApplyDamageEffect`
  (params (ch :type "BaseCharacter Object Reference"))
  (bind _returnvalue (`self.GetASC`))
  (`/Engine/EditorBlueprintResources/StandardMacros.IsValid` ch
    (:`Is Valid`
      (bind _returnvalue_2 (`AbilitySystemBlueprintLibrary.AssignTagSetByCallerMagnitude` (`AbilitySystemComponent.MakeOutgoingSpec` :`self` _returnvalue :`GameplayEffectClass` "/Game/ProjectAE/Blueprints/Abilities/GameplayEffects/Modify/GE_ApplyDamage.GE_ApplyDamage_C") (struct :`TagName` "Data.Damage") (`self.Magnitude`)))
      (`AbilitySystemComponent.BP_ApplyGameplayEffectSpecToTarget` _returnvalue _returnvalue_2 (`self.GetASC` ch)))))

(fn `PerformAttack`
  (bind _returnvalue (`self.K2_GetActorLocation`))
  (bind _returnvalue_2 (== (`self.SelectedSection`) "JumpAttack"))
  (bind _returnvalue_3 (+ (`self.K2_GetActorLocation`) (* (`self.GetActorForwardVector`) (+ (`self.AttackRange`) (`self.AcceptableAtkInterval`)))))
  (`parent.PerformAttack`)
  (if (not (`KismetArrayLibrary.Array_Contains` (`self.RangeAttacks`) (`self.SelectedSection`)))
    (bind (_outhit _returnvalue_4) (`KismetSystemLibrary.BoxTraceSingle` :`Start` _returnvalue :`End` (+ _returnvalue (* (`self.GetActorForwardVector`) (+ (`self.AttackRange`) (`self.AcceptableAtkInterval`)))) :`HalfSize` (50.0 50.0 50.0) :`TraceChannel` "TraceTypeQuery4" :`DrawDebugType` "ForDuration" :`DrawTime` 3.0))
    (if _returnvalue_4
      (bind _asplayer_character (cast `PlayerCharacter` (`.HitActor` (`GameplayStatics.BreakHitResult` _outhit)))
        (:`then`
          _)
        (:`CastFailed`
          (`AEGloabalHelper.PrintString` "플레이어 캐스트 실패" 5.0 (struct :`B` 255 :`G` 255 :`R` 255 :`A` 255))))
      (`self.ApplyDamageEffect` _asplayer_character))
    (else
      (`|ExecutionSequence`
        (:`then_0`
          (bind (_outhit_2 _returnvalue_5) (`KismetSystemLibrary.SphereTraceSingle` _returnvalue_3 _returnvalue_3 (`KismetMathLibrary.SelectFloat` 300.0 200.0 _returnvalue_2) "TraceTypeQuery4" false (`self.Actors to Ignore`) "ForDuration" true (struct :`R` 1.0 :`A` 1.0) (struct :`G` 1.0 :`A` 1.0) 3.0))
          (if _returnvalue_5
            (bind (_bblockinghit _binitialoverlap _time _distance _location _impactpoint _normal _impactnormal _physmat _hitactor) (`GameplayStatics.BreakHitResult` _outhit_2))
            (`KismetArrayLibrary.Array_AddUnique` (`self.Actors to Ignore`) _hitactor)
            (bind _asplayer_character_2 (cast `PlayerCharacter` _hitactor)
              (:`then`
                _)
              (:`CastFailed`
                (`AEGloabalHelper.PrintString` "플레이어 캐스트 실패" 5.0 (struct :`B` 255 :`G` 255 :`R` 255 :`A` 255))))
            (`self.ApplyDamageEffect` _asplayer_character_2)))
        (:`then_1`
          (if _returnvalue_2
            (`GameplayStatics.SpawnDecalAtLocation` (`self.GroundBrokenMaterialInst`) (512.0 512.0 512.0) _returnvalue_3 (struct :`Pitch` -90.0) 2.0)))))))

(fn `PlayAttackMontage`
  (bind _output_get (set `self.SelectedSection` (`|GetArrayItem` (select `bool` (> (`KismetMathLibrary.RandomFloat`) (`KismetMathLibrary.SelectFloat` 0.5 0.25 (>= (`self.GetDistanceTo` (`GameplayStatics.GetPlayerCharacter` 0)) (`self.AttackRange`)))) :`false` (`self.RangeAttacks`) :`true` (`self.CloseAttacks`)) (`KismetMathLibrary.RandomInteger` 2))))
  (`parent.PlayAttackMontage`))

(fn `ResetAttackCooldown`
  (`parent.ResetAttackCooldown`)
  (`KismetArrayLibrary.Array_Clear` (`self.Actors to Ignore`)))

(fn `SetMovementSpeed`
  (params (Speed :type "/Game/ProjectAE/AI/Enums/E_MovementSpeed Enum" :default "NewEnumerator0"))
  (returns (SpeedValue :type "Float (double-precision)"))
  (set `CharacterMovementComponent.MaxWalkSpeed` (select `/Game/ProjectAE/AI/Enums/E_MovementSpeed` Speed :`NewEnumerator1` 100.0 :`NewEnumerator2` 300.0 :`NewEnumerator3` 1000.0 :!type "Float (single-precision)") (`self.CharacterMovement`))
  (return 0.0))

(fn `UserConstructionScript`
  (`parent.UserConstructionScript`))