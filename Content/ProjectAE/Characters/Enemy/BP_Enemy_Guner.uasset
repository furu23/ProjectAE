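; BP_Enemy_Guner is a gun enemy whose ranged attack spawns an actor from its muzzle carrying GAS damage.
; PerformAttack calls the parent, then builds a GE_ApplyDamage spec with its magnitude set by caller through the Data.Damage tag.
; It spawns the actor at the Muzzle socket facing the enemy's forward vector, passing the spec along with itself as owner and instigator.
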(fn `PerformAttack`
  (`parent.PerformAttack`)
  (bind _returnvalue (`AbilitySystemBlueprintLibrary.AssignTagSetByCallerMagnitude` (`AbilitySystemComponent.MakeOutgoingSpec` :`self` (`self.GetASC`) :`GameplayEffectClass` "/Game/ProjectAE/Blueprints/Abilities/GameplayEffects/Modify/GE_ApplyDamage.GE_ApplyDamage_C") (struct :`TagName` "Data.Damage") (`self.Magnitude`)))
  (`|SpawnActorFromClass` "/Game/ProjectAE/Blueprints/Actors/Projectiles/BP_BulletDefault.BP_BulletDefault_C" (`KismetMathLibrary.MakeTransform` (`SceneComponent.GetSocketLocation` (`self.Mesh`) "Muzzle") (`KismetMathLibrary.MakeRotFromX` (`self.GetActorForwardVector`))) "Undefined" "MultiplyWithRoot" self _returnvalue self))

(fn `UserConstructionScript`
  (`parent.UserConstructionScript`))