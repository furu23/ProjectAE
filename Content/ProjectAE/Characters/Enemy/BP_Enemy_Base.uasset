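; Base enemy character paired with AIC_Enemy_Base, providing attacks, damage reactions, death and spline patrolling.
; Damage triggers aggro, sound, a material flash and DoOnce-gated hit reactions that briefly pause the AI brain.
; A rear sphere reports the player to the controller, and patrol helpers ping-pong along spline points.
; Attack montages use a timer cooldown synced to the Blackboard, while PerformAttack is an empty stub.
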(event `self.ReceivePossessed`
  (params (NewController :type "Controller Object Reference"))
  (bind _asaic_enemy_base (cast `/Game/ProjectAE/AI/AIC_Enemy_Base` NewController))
  (set `self.AIControllerRef` _asaic_enemy_base))

(event `self.OnDeath`
  (params (Causer :type "Actor Object Reference") (Victim :type "Actor Object Reference"))
  (`parent.OnDeath` Causer Victim)
  (`self.PlayDeathMontage`)
  (`/Game/ProjectAE/AI/AIC_Enemy_Base.OnDeath` (`self.AIControllerRef`))
  (`KismetSystemLibrary.Delay` 2.0)
  (`self.K2_DestroyActor`))

(event `self.ReceiveBeginPlay`
  (bind _mesh (`self.Mesh`))
  (`parent.ReceiveBeginPlay`)
  (bind _returnvalue (`PrimitiveComponent.CreateDynamicMaterialInstance` _mesh 0 (`PrimitiveComponent.GetMaterial` _mesh 0) "None"))
  (set `self.DynamicMat` _returnvalue))

(event `self.OnDamaged`
  (params (Causer :type "Actor Object Reference") (Victim :type "Actor Object Reference"))
  (`parent.OnDamaged` Causer Victim)
  (`|ExecutionSequence`
    (:`then_0`
      (if (<= (`HealthComponent.GetHealth1` (`self.HealthComp`)) 30.0)
        (`/Engine/EditorBlueprintResources/StandardMacros.DoOnce` false
          (:`Completed`
            (goto _label :!via `Reset`)))))
    (:`then_1`
      (`/Engine/EditorBlueprintResources/StandardMacros.DoOnce` false :!label _label
        (:`Completed`
          (`self.PlayDamagedMontage`)
          (bind _aicontrollerref (`self.AIControllerRef`)
            (:`then`
              (`Controller.StopMovement` _aicontrollerref)
              (bind _braincomponent (`AIController.BrainComponent` _aicontrollerref))
              (`ActorComponent.Deactivate` _braincomponent)
              (`KismetSystemLibrary.RetriggerableDelay` 1.0)
              (`ActorComponent.Activate` _braincomponent false))
            (:`else`)))))
    (:`then_2`
      (bind _state (`/Game/ProjectAE/AI/AIC_Enemy_Base.GetCurrentState` (`self.AIControllerRef`)))
      (switch `/Game/ProjectAE/AI/Enums/E_AIState` _state
        (:`NewEnumerator0`
          _)
        (:`NewEnumerator3`
          _)
        (:`NewEnumerator5`
          _))
      (`/Game/ProjectAE/AI/AIC_Enemy_Base.SetStateAsAttacking` (`self.AIControllerRef`) (`GameplayStatics.GetPlayerCharacter` 0)))
    (:`then_3`
      (`GameplayStatics.PlaySoundAtLocation` (`self.DamagedSound`) (`self.K2_GetActorLocation`) (struct) 1.0 1.0 0.0 null null null null)
      (bind (_direction _newtrack_0) (`Timeline|FadeFlash` :!via `PlayFromStart`)
        (:`Update`
          (`MaterialInstanceDynamic.SetScalarParameterValue` (`self.DynamicMat`) "FlashParam" (`KismetMathLibrary.FClamp` _newtrack_0 0.0 5.0)))))))

(event `/Game/ProjectAE/AI/BPI_EnemyAI.IncreasePatrolRouteSpline`
  (`self.IncreasementPatrolRoute`))

(event `self.BackDetectionSphere.OnComponentBeginOverlap`
  (params (OverlappedComponent :type "PrimitiveComponent Object Reference") (OtherActor :type "Actor Object Reference") (OtherComp :type "PrimitiveComponent Object Reference") (OtherBodyIndex :type Integer) (bFromSweep :type Boolean) (SweepResult :type "HitResult Structure (by ref)"))
  ;[0 0 0 1 24] 등 뒤 플레이어 감지 로직
  (cast `/Game/ProjectAE/Characters/Player/BP_Player` OtherActor)
  (bind _asaic_enemy_base (cast `/Game/ProjectAE/AI/AIC_Enemy_Base` (`self.GetController`)))
  (`/Game/ProjectAE/AI/AIC_Enemy_Base.HandleSensedSight` _asaic_enemy_base OtherActor))

(fn `FindNearPatrolRoute`
  (bind _patrol_route (`self.Patrol Route`)
    (:`then`
      (for _index (range (`/Game/ProjectAE/Characters/Enemy/BP_PatrolRoute.GetSplinePointsNum` _patrol_route))
        (bind _location (`/Game/ProjectAE/Characters/Enemy/BP_PatrolRoute.GetSplinePointAsWorldPosition` _patrol_route _index))
        (if (== _location (`SplineComponent.FindLocationClosestToWorldLocation` (`/Game/ProjectAE/Characters/Enemy/BP_PatrolRoute.PatrolRoute` _patrol_route) (`self.K2_GetActorLocation`) "World") :`ErrorTolerance` 0.1)
          (set `self.PatrolRouteIndex` _index)
          (break))))
    (:`else`)))

(fn `GetPatrolRoute`
  (returns (PatrolRoute :type "/Game/ProjectAE/Characters/Enemy/BP_PatrolRoute Object Reference"))
  (return (`self.Patrol Route`)))

(fn `GetPatrolRouteLocation`
  (returns (NewParam :type "Vector Structure"))
  (bind _patrol_route (`self.Patrol Route`)
    (:`then`
      (bind _location (`/Game/ProjectAE/Characters/Enemy/BP_PatrolRoute.GetSplinePointAsWorldPosition` _patrol_route (`self.PatrolRouteIndex`)))
      (return _location))
    (:`else`
      (return (`self.K2_GetActorLocation`)))))

(fn `IncreasementPatrolRoute`
  (bind _output_get (set `self.PatrolRouteIndex` (+ (`self.PatrolRouteIndex`) (`self.PatrolRouteDir`))))
  (if (>= _output_get (- (`/Game/ProjectAE/Characters/Enemy/BP_PatrolRoute.GetSplinePointsNum` (`self.Patrol Route`)) 1))
    (set `self.PatrolRouteDir` -1)
    (elif (<= (`self.PatrolRouteIndex`) 0)
      (set `self.PatrolRouteDir` 1))))

(fn `PerformAttack`)

(fn `PlayAttackMontage`
  (`/Engine/EditorBlueprintResources/StandardMacros.IsValid` (`self.AttackMontage          `)
    (:`Is Valid`
      (if (not (`self.bIsAttacking`))
        (`|ExecutionSequence`
          (:`then_0`
            (set `self.bIsAttacking` true))
          (:`then_1`
            (set `self.bCanAttack` false))
          (:`then_2`
            (`self.PlayAnimMontage` (`self.AttackMontage          `) 1.0 (`self.SelectedSection`))
            (bind _returnvalue (`KismetSystemLibrary.K2_SetTimer` null "ResetAttackCooldown" 2.0))
            (set `self.AttackCooldownTimer` _returnvalue)))))))

(fn `PlayDamagedMontage`
  (`self.PlayAnimMontage` (`self.HitReactMontage`)))

(fn `PlayDeathMontage`
  (`self.PlayAnimMontage` (`self.DeathMontage`)))

(fn `ResetAttackCooldown`
  (bind _returnvalue (`AIBlueprintHelperLibrary.GetBlackboard` (`AIBlueprintHelperLibrary.GetAIController` self)))
  (`/Engine/EditorBlueprintResources/StandardMacros.IsValid` _returnvalue
    (:`Is Valid`
      (bind _output_get (set `self.bCanAttack` true))
      (`BlackboardComponent.SetValueAsBool` _returnvalue "bCanAttack" _output_get)
      (bind _output_get_2 (set `self.bIsAttacking` false))
      (`BlackboardComponent.SetValueAsBool` _returnvalue "bIsAttacking" _output_get_2))))

(fn `SetMovementSpeed`
  (params (Speed :type "/Game/ProjectAE/AI/Enums/E_MovementSpeed Enum" :default "NewEnumerator0"))
  (returns (SpeedValue :type "Float (double-precision)"))
  (bind _output_get (set `CharacterMovementComponent.MaxWalkSpeed` (select `/Game/ProjectAE/AI/Enums/E_MovementSpeed` Speed :`NewEnumerator1` 100.0 :`NewEnumerator2` 300.0 :`NewEnumerator3` 500.0 :!type "Float (single-precision)") (`self.CharacterMovement`)))
  (return _output_get))

(fn `UserConstructionScript`)