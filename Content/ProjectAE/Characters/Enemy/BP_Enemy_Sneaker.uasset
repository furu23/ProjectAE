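; BP_Enemy_Sneaker is a melee enemy Blueprint that overrides its parent's attack and movement-speed behaviour.
; PlayAttackMontage picks a random montage section before deferring to the parent.
; PerformAttack runs a debug-drawn forward box trace in BaseAttack, then damages a hit PlayerCharacter through a GAS effect with SetByCaller magnitude.
; SetMovementSpeed maps idle, walking, jogging and sprinting states to max walk speed.
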(fn `ApplyDamage`
  (params (Object :type "Object Object Reference"))
  (bind _returnvalue (`self.GetASC`))
  (bind _asplayer_character (cast `PlayerCharacter` Object))
  (bind _returnvalue_2 (`AbilitySystemBlueprintLibrary.AssignTagSetByCallerMagnitude` (`AbilitySystemComponent.MakeOutgoingSpec` :`self` _returnvalue :`GameplayEffectClass` "/Game/ProjectAE/Blueprints/Abilities/GameplayEffects/Modify/GE_ApplyDamage.GE_ApplyDamage_C") (struct :`TagName` "Data.Damage") (`self.Magnitude`)))
  (`AbilitySystemComponent.BP_ApplyGameplayEffectSpecToTarget` _returnvalue _returnvalue_2 (`self.GetASC` _asplayer_character)))

(fn `PerformAttack`
  (bind _returnvalue (`self.K2_GetActorLocation`))
  (`parent.PerformAttack`)
  (bind (_outhit _returnvalue_2) (`KismetSystemLibrary.BoxTraceSingle` :`Start` _returnvalue :`End` (+ _returnvalue (* (`self.GetActorForwardVector`) (+ (`self.AttackRange            `) (`self.AcceptableAtkInterval`)))) :`HalfSize` (100.0 100.0 100.0) :`TraceChannel` "TraceTypeQuery4" :`DrawDebugType` "ForDuration" :`DrawTime` 3.0))
  (if _returnvalue_2
    (bind (_bblockinghit _binitialoverlap _time _distance _location _impactpoint _normal _impactnormal _physmat _hitactor) (`GameplayStatics.BreakHitResult` _outhit))
    (`AEGloabalHelper.PrintString` (`KismetSystemLibrary.GetDisplayName` _hitactor) 3.0 (make `Color` 0 0 255 255) true)
    (`self.ApplyDamage` _hitactor)))

(fn `PlayAttackMontage`
  (bind _output_get (set `self.SelectedSection` (`|GetArrayItem` (`self.AttackSections`) (`KismetMathLibrary.RandomInteger` 2))))
  (`parent.PlayAttackMontage`))

(fn `SetMovementSpeed`
  (params (Speed :type "/Game/ProjectAE/AI/Enums/E_MovementSpeed Enum" :default "NewEnumerator0"))
  (returns (SpeedValue :type "Float (double-precision)"))
  (bind _output_get (set `CharacterMovementComponent.MaxWalkSpeed` (select `/Game/ProjectAE/AI/Enums/E_MovementSpeed` Speed :`NewEnumerator1` 100.0 :`NewEnumerator2` 300.0 :`NewEnumerator3` 1000.0 :!type "Float (single-precision)") (`self.CharacterMovement`)))
  (return _output_get))

(fn `UserConstructionScript`
  (`parent.UserConstructionScript`))