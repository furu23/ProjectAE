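; Player character Blueprint that handles movement on world axes, interaction and rotation toward the cursor while aiming.
; BeginPlay disables controller yaw, shows the cursor in game-and-UI input mode and creates a HUD widget marked for later removal.
; Enhanced Input drives movement and InteractionComponent, whose focus changes toggle the HUD interaction prompt.
; Debug keys play fire and roll montages and add Wood or Rock to InventoryComponent.
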(event OnFocusChanged(InteractionComponent)
  (params (NewFocusedActor :type Actor%20Object%20Reference))
  (bind _testwidget (Variables|Default|GetTestWidget))
  (Utilities|IsValid NewFocusedActor
    (:Is%20Valid
      (Class|AEGameHUDWidget|ShowInteractionPrompt _testwidget))
    (:Is%20Not%20Valid
      (Class|AEGameHUDWidget|HideInteractionPrompt _testwidget))))

(event Input|EnhancedActionEvents|EnhancedInputActionIA_Interact
  (params (ActionValue :type Boolean) (ElapsedSeconds :type Float%20%28double-precision%29) (TriggeredSeconds :type Float%20%28double-precision%29) (InputAction :type Input%20Action%20Object%20Reference :default "/Game/ProjectAE/Data/Input/Actions/IA_Interact.IA_Interact"))
  (:Started
    (Class|InteractionComponent|TryInteract (Variables|Default|GetInteractionComponent))))

(event Input|EnhancedActionEvents|EnhancedInputActionIA_Move
  (params (ActionValue :type Vector%202D%20Structure) (ElapsedSeconds :type Float%20%28double-precision%29) (TriggeredSeconds :type Float%20%28double-precision%29) (InputAction :type Input%20Action%20Object%20Reference :default "/Game/ProjectAE/Data/Input/Actions/IA_Move.IA_Move"))
  (Pawn|Input|AddMovementInput (Math|Conversions|ToVector(Vector2D) ActionValue) 1.0 false))

(event EventBeginPlay
  (bind _returnvalue (Game|GetPlayerController 0))
  (|CallParentFunction)
  (Variables|Default|SetbUseControllerRotationYaw false)
  ;[1 0 0] 추후에 제거 예정
  (bind _returnvalue_2 (UserInterface|CreateWidget "/Game/ProjectAE/Widgets/WBP_HUDWidget.WBP_HUDWidget_C"))
  (UserInterface|Viewport|AddtoViewport _returnvalue_2 0)
  (Variables|Default|SetTestWidget _returnvalue_2)
  (Variables|/Script/Engine.PlayerController|SetbShowMouseCursor _returnvalue true)
  (Input|SetInputModeGameandUI _returnvalue 0 "DoNotLock" false false))

(event EventTick
  (params (DeltaSeconds :type Float%20%28single-precision%29))
  (if (Variables|Default|GetbIsAiming)
    (Class|PlayerCharacter|RotatetoCursor)))

(event Input|MouseEvents|DebugKeyLeftMouseButton
  (params (Key :type Key%20Structure) (ActionValue :type Input%20Action%20Value%20Structure))
  (:Pressed
    (Animation|PlayAnimMontage "/Game/RadicalMike/Animations/Anim_ZMIKE_FireR_Montage.Anim_ZMIKE_FireR_Montage" 1.0 "None")))

(event Input|KeyboardEvents|DebugKeyT
  (params (Key :type Key%20Structure) (ActionValue :type Input%20Action%20Value%20Structure))
  (:Pressed
    (Animation|PlayAnimMontage "/Game/RadicalMike/Mixamo/Retargeting/Sprinting_Forward_Roll_Anim_Modified_Montage.Sprinting_Forward_Roll_Anim_Modified_Montage" 1.0 "None")))

(event Input|KeyboardEvents|DebugKey1
  (params (Key :type Key%20Structure) (ActionValue :type Input%20Action%20Value%20Structure))
  ;[1 0 0] Debug 용 테스트 키 입니당
  (:Pressed
    (Class|InventoryComponent|AddItem (Variables|Default|GetInventoryComponent) "Wood" 10 (Variables|Default|GetOut%20Remaining%20Amount))))

(event Input|KeyboardEvents|DebugKey2
  (params (Key :type Key%20Structure) (ActionValue :type Input%20Action%20Value%20Structure))
  ;[1 0 0] Debug 용 테스트 키 입니당
  (:Pressed
    (Class|InventoryComponent|AddItem (Variables|Default|GetInventoryComponent) "Rock" 10 (Variables|Default|GetOut%20Remaining%20Amount))))

(fn ConstructionScript)