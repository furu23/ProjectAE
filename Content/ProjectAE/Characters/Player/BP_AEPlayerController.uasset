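; Player controller that builds the gameplay UI, binding skill, health, bio and ammo widgets to the Ability System Component and weapon.
; Each tick it turns control rotation toward the cursor's hit point, with a crosshair cursor widget that changes on look input.
; Game phase changes drive a fade overlay for loading and in-game, and a save in post-game.
; Inputs toggle pause, quest and inventory UI.
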(event Custom|OnQuestNPCInteract)

(event Custom|SetSystemCursorDefault
  ;[0 0 0 1 24] SetInputMode + 커서 변경
  (Variables|Default|SetCurrentMouseCursor "Default"))

(event Custom|SetSystemCursorCrosshairs
  ;[0 0 0 1 24] SetInputMode + 커서 변경
  (Variables|Default|SetCurrentMouseCursor "Crosshairs"))

(event Custom|SetCursorToDefault
  ;[0 0 0 1 24] SetInputMode + 커서 변경
  (bind _crosshairwidget (Variables|Default|GetCrosshairWidget)
    (:then
      (Default|SetCursortoDefault _crosshairwidget))
    (:else)))

(event Custom|SetCursorToFocus
  ;[0 0 0 1 24] SetInputMode + 커서 변경
  (bind _crosshairwidget (Variables|Default|GetCrosshairWidget)
    (:then
      (Default|SetCursortoFocus _crosshairwidget))
    (:else)))

(event Custom|SetAEInputMode
  ;[0 0 0 1 24] SetInputMode + 커서 변경
  (Input|SetInputModeGameandUI self 0 "DoNotLock" false false)
  (Variables|Default|SetbShowMouseCursor true)
  (CallFunction|SetSystemCursorCrosshairs))

(event Custom|OnPhaseChanged
  (params (NewPhase :type Gameplay%20Tag%20Structure))
  ;[0.3124 1 0.9901] 코어 게임 흐름 관련
  (|SwitchGameplayTag NewPhase
    (:Game.Phase.Loading
      (CallFunction|CurrentlyDoNothing) ; Loading Phase는 현재 매우 짧으므로. 특별히 필요할 때 이용해주세요.\n식생 로딩까지 넉넉히 로딩을 추가할 경우 사용 여지가 커집니다.
    )
    (:Game.Phase.InGame
      (CallFunction|OninGameStateStarted) ; TODO: 효과 및 UI 등 필요한 것들을 여기 세팅
    )
    (:Game.Phase.PostGame
      (CallFunction|OnPostGameStateStarted) ; TODO: UI 생성, 조작 및 소리 등 조절
    )))

(event Custom|TogglePauseGame
  (bind _aswbp_hudwidget (Utilities|Casting|CastToWBP_HUDWidget (Variables|Default|GetAEGameHUDWidget)))
  (Default|TogglePauseGame _aswbp_hudwidget))

(event Custom|RemoveSettingTag
  (Ability|GameplayEffect|RemoveLooseGameplayTags (Game|GetPlayerState 0) (Variables|Default|GetGameplay%20Tags)))

(event Custom|AddSettingTag
  (Ability|GameplayEffect|AddLooseGameplayTags (Game|GetPlayerState 0) (Variables|Default|GetGameplay%20Tags)))

(event Input|EnhancedActionEvents|EnhancedInputActionIA_Inventory
  (params (ActionValue :type Boolean) (ElapsedSeconds :type Float%20%28double-precision%29) (TriggeredSeconds :type Float%20%28double-precision%29) (InputAction :type Input%20Action%20Object%20Reference :default "/Game/ProjectAE/Data/Input/Actions/IA_Inventory.IA_Inventory"))
  (bind _inventoryuimanager (Variables|Default|GetInventoryUIManager))
  (:Started
    (if (Variables|/Script/ProjectAE.InventoryUIManager|GetbIsPlayerInventoryOpen _inventoryuimanager)
      (Class|InventoryUIManager|CloseAllInventories _inventoryuimanager)
      (else
        (Class|InventoryUIManager|OpenPlayerInventory _inventoryuimanager)))))

(event Input|EnhancedActionEvents|EnhancedInputActionIA_Quest
  (params (ActionValue :type Boolean) (ElapsedSeconds :type Float%20%28double-precision%29) (TriggeredSeconds :type Float%20%28double-precision%29) (InputAction :type Input%20Action%20Object%20Reference :default "/Game/ProjectAE/Data/Input/Actions/IA_Quest.IA_Quest"))
  (:Started
    (Class|AEGameHUDWidget|ToggleQuestWidget (Variables|Default|GetAEGameHUDWidget))))

(event Input|EnhancedActionEvents|EnhancedInputActionIA_Look
  (params (ActionValue :type Boolean) (ElapsedSeconds :type Float%20%28double-precision%29) (TriggeredSeconds :type Float%20%28double-precision%29) (InputAction :type Input%20Action%20Object%20Reference :default "/Game/ProjectAE/Data/Input/Actions/IA_Look.IA_Look"))
  (:Started
    (CallFunction|SetCursortoFocus))
  (:Canceled
    (CallFunction|SetCursortoDefault :!label _label))
  (:Completed
    (goto _label)))

(event EventBeginPlay
  (bind _returnvalue (UserInterface|CreateWidget "/Game/ProjectAE/Widgets/WBP_UIContainer.WBP_UIContainer_C" self))
  (UserInterface|Viewport|AddtoViewport _returnvalue 0)
  (CallFunction|UIAbilityBindInitialize _returnvalue (|GetASC))
  (CallFunction|InitializeCursor)
  (EventDispatchers|BindEventtoOnGamePhaseChangeDelegate (Subsystems|GetGamePhaseSubsystem) (EventDispatchers|CreateEvent :!event Custom|OnPhaseChanged)))

(event EventTick
  (params (DeltaSeconds :type Float%20%28single-precision%29))
  (Pawn|SetControlRotation (Math|Rotator|FindLookatRotation (Transformation|GetActorLocation (Pawn|GetControlledPawn)) (.location (.HitResult (Game|Player|GetHitResultUnderCursorbyChannel "TraceTypeQuery1" true))))))

(event EventPossess
  (params (PossessedPawn :type Pawn%20Object%20Reference))
  (|CallParentFunction PossessedPawn)
  (CallFunction|SetAEInputMode))

(event EventShowFadeAnim
  (params (PlayMode :type EUMGSequencePlayMode%20Enum :default "Forward"))
  ;[0 0 0 1 24] Interface
  (CallFunction|PlayFadeAnim PlayMode))

(event EventSetNormalInputMode
  ;[0 0 0 1 24] Interface
  (CallFunction|SetAEInputMode))

(event Input|KeyboardEvents|DebugKey8
  (params (Key :type Key%20Structure :default "None") (ActionValue :type Input%20Action%20Value%20Structure))
  ;[0 0 0 1 24] SetInputMode + 커서 변경
  (:Pressed
    (bind _crosshairwidget (Variables|Default|GetCrosshairWidget)
      (:then
        (Default|SetCursortoDefault _crosshairwidget))
      (:else))))

(event Input|KeyboardEvents|DebugKey9
  (params (Key :type Key%20Structure :default "None") (ActionValue :type Input%20Action%20Value%20Structure))
  ;[0 0 0 1 24] SetInputMode + 커서 변경
  (:Pressed
    (bind _crosshairwidget (Variables|Default|GetCrosshairWidget)
      (:then
        (Default|SetCursortoFocus _crosshairwidget))
      (:else))))

(event Input|KeyboardEvents|DebugKeyU
  (params (Key :type Key%20Structure :default "None") (ActionValue :type Input%20Action%20Value%20Structure))
  (:Pressed
    (bind _aswbp_hudwidget (Utilities|Casting|CastToWBP_HUDWidget (Variables|Default|GetAEGameHUDWidget)))
    (Default|TogglePauseGame _aswbp_hudwidget)))

(event Input|KeyboardEvents|Escape
  (params (Key :type Key%20Structure :default "None"))
  (:Pressed
    (bind _aswbp_hudwidget (Utilities|Casting|CastToWBP_HUDWidget (Variables|Default|GetAEGameHUDWidget)))
    (Default|TogglePauseGame _aswbp_hudwidget)))

(fn ConstructionScript)

(fn UIAbilityBindInitialize
  (params (Widget :type WBP%20UI%20Container%20Object%20Reference) (ASC :type Ability%20System%20Component%20Object%20Reference))
  (bind _returnvalue (Pawn|GetControlledPawn))
  (Class|SkillSlotWidget|BindtoASC (Variables|/Game/ProjectAE/Widgets/WBP_UIContainer.WBP_UIContainer_C|GetSkillSlot_1 Widget) ASC "(TagName=\"Cooldown.Skill.Repair\")")
  (Class|SkillSlotWidget|BindtoASC (Variables|/Game/ProjectAE/Widgets/WBP_UIContainer.WBP_UIContainer_C|GetSkillSlot_2 Widget) ASC "(TagName=\"Cooldown.Skill.Heist\")")
  (Class|SkillSlotWidget|BindtoASC (Variables|/Game/ProjectAE/Widgets/WBP_UIContainer.WBP_UIContainer_C|GetSkillSlot_3 Widget) ASC "(TagName=\"Cooldown.Skill.OverHeating\")")
  (Class|SkillSlotWidget|BindtoASC (Variables|/Game/ProjectAE/Widgets/WBP_UIContainer.WBP_UIContainer_C|GetSkillSlot_4 Widget) ASC "(TagName=\"Cooldown.Skill.Shockwave\")")
  (Class|StatBarWidgetBase|BindtoASC (Variables|/Game/ProjectAE/Widgets/WBP_UIContainer.WBP_UIContainer_C|GetHealthBar Widget) ASC)
  (Class|StatBarWidgetBase|BindtoASC (Variables|/Game/ProjectAE/Widgets/WBP_UIContainer.WBP_UIContainer_C|GetBioRadialBar Widget) ASC)
  (Utilities|IsValid _returnvalue
    (:Is%20Valid
      (bind _asbp_player (Utilities|Casting|CastToBP_Player _returnvalue))
      (Class|AmmoWidgetBase|InitializeWidget (Variables|/Game/ProjectAE/Widgets/WBP_UIContainer.WBP_UIContainer_C|GetAmmoWidget Widget) (Variables|/Script/ProjectAE.PlayerCharacter|GetWeaponComponent _asbp_player) ASC))))

(fn InitializeCursor
  (bind _returnvalue (UserInterface|CreateWidget "/Game/ProjectAE/Widgets/Cursor/WBP_Cursor_Crosshair.WBP_Cursor_Crosshair_C" self))
  (bind _output_get (Variables|Default|SetCrosshairWidget _returnvalue))
  (Class|PlayerController|SetMouseCursorWidget "Crosshairs" _output_get))

(fn CurrentlyDoNothing
  (bind _returnvalue (UserInterface|CreateWidget "/Game/ProjectAE/Widgets/WBP_Fade.WBP_Fade_C" self))
  (UserInterface|Viewport|AddtoViewport _returnvalue 99)
  (Variables|Default|SetFadeWidget _returnvalue))

(fn OnPostGameStateStarted
  (Class|SaveGameSubsystem|SaveGame (Subsystems|GetSaveGameSubsystem) false) ; 현재 위치는 여기지만, 동기식이므로 추후엔\n로딩 스크린을 띄운 상태거나 검은 화면일때 호출하는 식으로 옮겨주세요
)

(fn OninGameStateStarted
  (bind _fadewidget (Variables|Default|GetFadeWidget)
    (:then
      (Default|FadeAnim _fadewidget "Reverse"))
    (:else)))

(fn PlayFadeAnim
  (params (PlayMode :type EUMGSequencePlayMode%20Enum :default "Forward"))
  (Variables|Default|GetFadeWidget
    (:then
      _)
    (:else
      (bind _returnvalue (UserInterface|CreateWidget "/Game/ProjectAE/Widgets/WBP_Fade.WBP_Fade_C" self (Utilities|Select :Index PlayMode :Forward 1.0 :Reverse -1.0 :PingPong 0.0)))
      (Variables|Default|SetFadeWidget _returnvalue)))
  (if (UserInterface|Viewport|IsinViewport (Variables|Default|GetFadeWidget))
    _
    (else
      (UserInterface|Viewport|AddtoViewport (Variables|Default|GetFadeWidget) 99)))
  (Default|FadeAnim (Variables|Default|GetFadeWidget) PlayMode)
  (Input|SetInputModeUIOnly self 0 "DoNotLock" false)
  (Variables|Default|SetbShowMouseCursor false))

(fn ToggleSettingTag
  (bind _returnvalue (Game|GetPlayerState 0))
  (bind _gameplay_tags (Variables|Default|GetGameplay%20Tags))
  (if (GameplayTags|HasMatchingGameplayTag (Ability|GetAbilitySystemComponent _returnvalue) "(TagName=\"State.Config.OnSetting\")")
    (Ability|GameplayEffect|RemoveLooseGameplayTags _returnvalue _gameplay_tags)
    (else
      (Ability|GameplayEffect|AddLooseGameplayTags _returnvalue _gameplay_tags))))