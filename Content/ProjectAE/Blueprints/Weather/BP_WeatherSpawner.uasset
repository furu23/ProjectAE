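; Weather spawner actor that follows the player and plays the current weather's Niagara effect and looping or one-shot sound.
; On BeginPlay it requests a precipitation type (PTY) for a fixed grid point from a weather API and maps the code to one of three weather states.
; SetWeather ignores repeats, clears the old effect, then applies the matching data entry with audio fades.
; Debug keys Z, X and C force each state.
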(event Custom|OnReceivedPTY
  (params (PTYValue :type Integer) (bIsSuccess :type Boolean) (ErrorMessage :type String) (RawResult :type Current%20Weather%20Result%20Structure%20%28by%20ref%29))
  (bind _returnvalue (Utilities|Select :Index PTYValue :Option%200 "NewEnumerator0" :Option%201 "NewEnumerator1" :Option%202 "NewEnumerator2" :Option%203 "NewEnumerator2" :Option%204 "NewEnumerator1" :Option%205 "NewEnumerator1" :Option%206 "NewEnumerator1" :Option%207 "NewEnumerator2"))
  (if bIsSuccess
    (Development|PrintString "OnReceivedSuccess")
    (Development|PrintString (Utilities|String|EnumtoString _returnvalue))
    (CallFunction|SetWeather _returnvalue)
    (else
      (Development|PrintString ErrorMessage true true "(R=1.000000,G=0.000000,B=0.000000,A=1.000000)"))))

(event EventBeginPlay
  (bind _output_get (Variables|Default|SetPlayerRef (Game|Player|GetPlayerPawn 0)))
  (Input|EnableInput (Game|GetPlayerController 0) :!pinned true) ; Debug
  (Class|WeatherBPLibrary|GetPTY (Variables|Default|GetWeatherAPIKey) 55 127 (EventDispatchers|CreateEvent :!event Custom|OnReceivedPTY)))

(event EventTick
  (params (DeltaSeconds :type Float%20%28single-precision%29))
  (bind _playerref (Variables|Default|GetPlayerRef)
    (:then
      (Transformation|SetActorLocation (Math|Interpolation|VInterpTo (Transformation|GetActorLocation) (Transformation|GetActorLocation _playerref) DeltaSeconds 1e+01) false false))
    (:else)))

(event Input|KeyboardEvents|DebugKeyZ
  (params (Key :type Key%20Structure :default "None") (ActionValue :type Input%20Action%20Value%20Structure))
  ;[1 0 0 1 24] Debug
  (:Pressed
    (CallFunction|SetWeather "NewEnumerator0")))

(event Input|KeyboardEvents|DebugKeyX
  (params (Key :type Key%20Structure :default "None") (ActionValue :type Input%20Action%20Value%20Structure))
  ;[1 0 0 1 24] Debug
  (:Pressed
    (CallFunction|SetWeather "NewEnumerator1")))

(event Input|KeyboardEvents|DebugKeyC
  (params (Key :type Key%20Structure :default "None") (ActionValue :type Input%20Action%20Value%20Structure))
  ;[1 0 0 1 24] Debug
  (:Pressed
    (CallFunction|SetWeather "NewEnumerator2")))

(fn ConstructionScript)

(fn SetWeather
  (params (TargetKey :type EWeatherType%20Enum :default "NewEnumerator0"))
  (bind _currentweatherdata (Variables|Default|GetCurrentWeatherData))
  (bind _niagara (Variables|Default|GetNiagara))
  (bind _currentweatherdata_2 (Variables|Default|GetCurrentWeatherData))
  (bind _audio (Variables|Default|GetAudio))
  (if (Utilities|Enum|Equal(Enum) TargetKey (Variables|Default|GetCurrentKey))
    (return)
    (else
      (CallFunction|ClearWeather)
      (CallFunction|SetCurrentWeatherData TargetKey)
      (Utilities|FlowControl|Sequence
        (:then_0
          ;[0 0 0] Particle
          (Utilities|IsValid (.particlesystem (Variables|Default|GetCurrentWeatherData))
            (:Is%20Valid
              (if (Components|Activation|IsActive _niagara)
                _
                (else
                  (Components|Activation|Activate _niagara false)))
              (Class|NiagaraComponent|SetAsset _niagara (.particlesystem _currentweatherdata) true)
              (Niagara|SetNiagaraVariable(Float) _niagara "Amount" (.amount _currentweatherdata)))))
        (:then_1
          ;[0 0 0] Audio
          (Utilities|IsValid (.soundeffect _currentweatherdata_2)
            (:Is%20Valid
              (Audio|Components|Audio|SetSound _audio (.soundeffect _currentweatherdata_2))
              (Audio|Components|Audio|FadeIn _audio 1.0 1.0 0.0 "Linear" :!class /Script/Engine.AudioComponent))))))))

(fn ClearWeather
  (Components|Activation|Deactivate (Variables|Default|GetNiagara))
  (Audio|Components|Audio|FadeOut (Variables|Default|GetAudio) 1.0 0.0 "Linear" :!class /Script/Engine.AudioComponent))

(fn SetCurrentWeatherData
  (params (TargetKey :type EWeatherType%20Enum :default "NewEnumerator0"))
  (Variables|Default|SetCurrentKey TargetKey)
  (bind _array_element (Utilities|Array|ForEachLoopwithBreak (Variables|Default|GetWeatherDatas) :!label _label)
    (:LoopBody
      (if (Utilities|Enum|Equal(Enum) TargetKey (.Key (Utilities|Struct|BreakFWeatherData _array_element)))
        (Variables|Default|SetCurrentWeatherData _array_element)
        (goto _label Break)))
    (:Completed
      (return))))