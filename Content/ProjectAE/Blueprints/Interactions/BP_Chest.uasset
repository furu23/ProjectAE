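; Interactable chest that fills its inventory with spawned items at BeginPlay through its RandomItemSpawn reference.
; Interacting while closed marks it open and passes its inventory to the InventoryUIManager on player controller 0, regardless of the caller.
; The inventory's closed event resets the chest so it can be used again.
; Open and close only toggle IsOpen, with animation left as a placeholder comment.
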(event `self.ReceiveBeginPlay`
  (`parent.ReceiveBeginPlay`)
  (bind _inventory (`self.Inventory`)
    (:`then`
      (bind _randomitemspawn (`self.RandomItemSpawn`)
        (:`then`
          (`RandomItemSpawnComponent.SpawnItemsIntoInventory` _randomitemspawn _inventory))
        (:`else`)))
    (:`else`)))

(event `self.OnInteract`
  (params (Caller :type "Actor Object Reference"))
  (if (not (`self.bIsOpen`))
    (`parent.OnInteract` Caller)
    (`self.OpenChest`)
    (bind _asbp_aeplayer_controller (cast `/Game/ProjectAE/Characters/Player/BP_AEPlayerController` (`GameplayStatics.GetPlayerController` 0)))
    (bind _returnvalue (`self.GetComponentByClass` _asbp_aeplayer_controller "/Script/ProjectAE.InventoryUIManager"))
    (`/Engine/EditorBlueprintResources/StandardMacros.IsValid` _returnvalue
      (:`Is Valid`
        (`InventoryUIManager.OpenChestInventory` _returnvalue (`self.GetChestInventory`))))))

(event `self.Inventory.OnInventoryClosed`
  (`self.CloseChest`))

(event `OpenChest`
  (set `self.bIsOpen` true))

(event `CloseChest`
  (set `self.bIsOpen` false))

(fn `GetChestInventory`
  (returns (ChestInventory :type "InventoryComponent Object Reference"))
  (return (`self.Inventory`)))

(fn `UserConstructionScript`
  (`parent.UserConstructionScript`))