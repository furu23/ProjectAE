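; BP_AEHUD is the game's HUD actor, linking the game HUD widget and the mouse cursor to the player controller.
; On BeginPlay it caches the first BP_AEPlayerController and sets it as the owning player of GameHUDWidget.
; Widget open events switch that controller to the default system cursor and play an open sound, while close events restore the crosshair cursor.
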(event `self.ReceiveBeginPlay`
  (bind _asbp_aeplayer_controller (cast `/Game/ProjectAE/Characters/Player/BP_AEPlayerController` (`GameplayStatics.GetPlayerController` 0)))
  (bind _output_get (set `self.AEPlayerControllerRef` _asbp_aeplayer_controller))
  (`UserWidget.SetOwningPlayer` (`self.GameHUDWidget`) _output_get))

(event `self.OnWidgetOpened`
  (bind _aeplayercontrollerref (`self.AEPlayerControllerRef`)
    (:`then`
      (`/Game/ProjectAE/Characters/Player/BP_AEPlayerController.SetSystemCursorDefault` _aeplayercontrollerref)
      (`GameplayStatics.PlaySound2D` "/Engine/VREditor/Sounds/VR_open_Cue.VR_open_Cue" 1.0 1.0 0.0 null null))
    (:`else`)))

(event `self.OnWidgetClosed`
  (bind _aeplayercontrollerref (`self.AEPlayerControllerRef`)
    (:`then`
      (`/Game/ProjectAE/Characters/Player/BP_AEPlayerController.SetSystemCursorCrosshairs` _aeplayercontrollerref))
    (:`else`)))

(fn `UserConstructionScript`)