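; Gameplay ability that reloads the player's weapon.
; On activation it plays a montage and spawns an effect at the mesh's right buster socket transform.
; Completion removes the DrainAmmo condition effect, calls ReloadWeapon on the AEWeaponComponent of the character found through the owning PlayerState, then ends.
; Blend out, interruption or cancellation destroys the effect and ends the ability only if that effect is still valid.
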(event `self.K2_ActivateAbility`
  (bind (_returnvalue_owneractor _returnvalue_avataractor) (break `GameplayAbilityActorInfo` (`self.GetActorInfo`)))
  (bind _reloadeffect (`self.ReloadEffect`))
  (bind _asplayer_character (`self.GetCharacter`))
  (`AbilityTask_PlayMontageAndWait.CreatePlayMontageAndWaitProxy` "Reload" null 0.5
    (:`then`
      (bind _asbp_player (cast `/Game/ProjectAE/Characters/Player/BP_Player` _returnvalue_avataractor))
      (bind (_returnvalue_location _returnvalue_rotation _returnvalue_scale) (`KismetMathLibrary.BreakTransform` (`SceneComponent.GetSocketTransform` (`Character.Mesh` _asbp_player) "Buster_RSocket" "RTS_World")))
      (bind _returnvalue (`NiagaraFunctionLibrary.SpawnSystemAtLocation` null _returnvalue_location _returnvalue_rotation _returnvalue_scale))
      (set `self.ReloadEffect` _returnvalue))
    (:`OnCompleted`
      (`self.BP_RemoveGameplayEffectFromOwnerWithGrantedTags` (struct :`GameplayTags` (struct :`(TagName` "State.Condition.DrainAmmo"))))
      (`AEWeaponComponent.ReloadWeapon` (`Actor.GetComponentByClass` _asplayer_character "/Script/ProjectAE.AEWeaponComponent"))
      (`self.K2_EndAbility`))
    (:`OnBlendOut`
      (`/Engine/EditorBlueprintResources/StandardMacros.IsValid` _reloadeffect :!label _label
        (:`Is Valid`
          (`ActorComponent.K2_DestroyComponent` _reloadeffect)
          (`self.K2_EndAbility`))))
    (:`OnInterrupted`
      (goto _label))
    (:`OnCancelled`
      (goto _label))))

(fn `GetCharacter`
  (returns (`AsPlayer Character` :type "PlayerCharacter Object Reference"))
  (bind _asplayer_state (cast `PlayerState` (`self.GetOwningActorFromActorInfo`))
    (:`then`
      (bind _asplayer_character (cast `PlayerCharacter` (`PlayerState.GetPawn` _asplayer_state))))
    (:`CastFailed`
      _))
  (return _asplayer_character))