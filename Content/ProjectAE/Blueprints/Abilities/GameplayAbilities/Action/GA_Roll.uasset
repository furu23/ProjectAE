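; GA_Roll is a gameplay ability that makes player character 0 perform a forward roll.
; It commits only the cooldown, snaps yaw to the last movement input if nonzero, then plays a sped-up roll montage.
; The ability ends itself only on montage completion, and OnEndAbility applies GE_RegenationBlock to the owner whether cancelled or not.
; A roll sound node exists but is not connected.
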(event `self.K2_ActivateAbility`
  (bind _returnvalue (`GameplayStatics.GetPlayerCharacter` 0))
  (bind _returnvalue_2 (`Pawn.GetLastMovementInputVector` _returnvalue))
  (bind (_returnvalue_roll _returnvalue_pitch _returnvalue_yaw) (`KismetMathLibrary.BreakRotator` (`KismetMathLibrary.Conv_VectorToRotator` _returnvalue_2)))
  (`parent.K2_ActivateAbility`)
  (`self.K2_CommitAbilityCooldown` false)
  (if (not (`KismetMathLibrary.Vector_IsNearlyZero` _returnvalue_2))
    (`Actor.K2_SetActorRotation` _returnvalue (`KismetMathLibrary.MakeRotator` 0.0 0.0 _returnvalue_yaw) false))
  (`|PlayMontage` (`Actor.GetComponentByClass` _returnvalue "/Script/Engine.SkeletalMeshComponent") "/Game/RadicalMike/Mixamo/Retargeting/Sprinting_Forward_Roll_Anim_Modified_Montage.Sprinting_Forward_Roll_Anim_Modified_Montage" 1.5
    (:`OnCompleted`
      (`self.K2_EndAbility`))))

(event `self.K2_OnEndAbility`
  (params (bWasCancelled :type Boolean))
  (`self.BP_ApplyGameplayEffectToOwner` "/Game/ProjectAE/Blueprints/Abilities/GameplayEffects/State/GE_RegenationBlock.GE_RegenationBlock_C")
  (`parent.K2_OnEndAbility` bWasCancelled))