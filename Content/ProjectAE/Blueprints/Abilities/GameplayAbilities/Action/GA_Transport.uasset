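; GA_Transport is a gameplay ability that teleports the player after a sped-up forward-roll montage.
; When the montage completes, it gets BP_Player through the owning AEPlayerState, moves the pawn without sweep, then ends.
; GetTargetLocation supplies the destination, but its forward-offset calculation from the player's target rotation appears unconnected.
; Only montage completion is handled, so interruption or cancellation does not reach EndAbility.
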(event `self.K2_ActivateAbility`
  (`AbilityTask_PlayMontageAndWait.CreatePlayMontageAndWaitProxy` "Teleport" "/Game/RadicalMike/Mixamo/Retargeting/Sprinting_Forward_Roll_Anim_Modified_Montage.Sprinting_Forward_Roll_Anim_Modified_Montage" 2.0
    (:`OnCompleted`
      (bind _asaeplayer_state (cast `AEPlayerState` (`self.GetOwningActorFromActorInfo`)))
      (bind _asbp_player (cast `/Game/ProjectAE/Characters/Player/BP_Player` (`PlayerState.GetPawn` _asaeplayer_state)))
      (`Actor.K2_SetActorLocation` _asbp_player (`self.GetTargetLocation` _asbp_player) false true)
      (`self.K2_EndAbility`))))