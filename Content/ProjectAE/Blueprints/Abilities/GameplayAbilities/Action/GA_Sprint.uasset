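; Sprint gameplay ability that raises the character's walk speed while the Input.Sprint tag is held.
; It reaches the Character through the owning PlayerState's pawn and adds a flat bonus to GetMaxSpeed, writing the result to MaxWalkSpeed.
; A tag-removal task ends the ability, and OnEndAbility subtracts the same amount from the current max speed, then applies GE_RegenationBlock to the owner.
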(event `self.K2_ActivateAbility`
  (`parent.K2_ActivateAbility`)
  (`AbilityTask_WaitGameplayTagRemoved.WaitGameplayTagRemove` (struct :`TagName` "Input.Sprint") null
    (:`then`
      (bind _asplayer_state (cast `PlayerState` (`self.GetOwningActorFromActorInfo`)))
      (bind _ascharacter (cast `Character` (`PlayerState.GetPawn` _asplayer_state)))
      (bind _charactermovement (`Character.CharacterMovement` _ascharacter))
      (set `CharacterMovementComponent.MaxWalkSpeed` (+ (`MovementComponent.GetMaxSpeed` _charactermovement) 500.0) _charactermovement))
    (:`Removed`
      (`self.K2_EndAbility`))))

(event `self.K2_OnEndAbility`
  (params (bWasCancelled :type Boolean))
  (bind _asplayer_state (cast `PlayerState` (`self.GetOwningActorFromActorInfo`)))
  (bind _ascharacter (cast `Character` (`PlayerState.GetPawn` _asplayer_state)))
  (bind _charactermovement (`Character.CharacterMovement` _ascharacter))
  (set `CharacterMovementComponent.MaxWalkSpeed` (+ (`MovementComponent.GetMaxSpeed` _charactermovement) -500.0) _charactermovement)
  (`self.BP_ApplyGameplayEffectToOwner` "/Game/ProjectAE/Blueprints/Abilities/GameplayEffects/State/GE_RegenationBlock.GE_RegenationBlock_C")
  (`parent.K2_OnEndAbility` bWasCancelled))