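; Repair skill Gameplay Ability that restores health to its owner.
; On activation it plays a montage and attaches a Niagara effect to the BP_Player capsule.
; On blend out or completion, it applies GE_RepairHealth through SetByCaller tag Data.Damage, capping the amount at the gap between two attributes or a fixed maximum.
; It then commits cooldown and ends, while interruption or cancellation ends it without healing or cooldown.
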(event `self.K2_ActivateAbility`
  (bind (_returnvalue_owneractor _returnvalue_avataractor _returnvalue_playercontroller _returnvalue_abilitysystemcomponent) (break `GameplayAbilityActorInfo` (`self.GetActorInfo`)))
  (bind _returnvalue (`self.MakeOutgoingGameplayEffectSpec` "/Game/ProjectAE/Blueprints/Abilities/GameplayEffects/Modify/GE_RepairHealth.GE_RepairHealth_C"))
  (bind (_bfound _returnvalue_2) (`AbilitySystemComponent.GetGameplayAttributeValue` _returnvalue_abilitysystemcomponent (struct :`AttributeName` "MaxHealth" :`Attribute` "/Script/ProjectAE.AS_HealthSet:MaxHealth" :`AttributeOwner` "/Script/CoreUObject.Class'/Script/ProjectAE.AS_HealthSet'")))
  (bind (_bfound_2 _returnvalue_3) (`AbilitySystemComponent.GetGameplayAttributeValue` _returnvalue_abilitysystemcomponent (struct :`AttributeName` "Health" :`Attribute` "/Script/ProjectAE.AS_HealthSet:Health" :`AttributeOwner` "/Script/CoreUObject.Class'/Script/ProjectAE.AS_HealthSet'")))
  (bind _returnvalue_4 (- _returnvalue_2 _returnvalue_3))
  (`AbilityTask_PlayMontageAndWait.CreatePlayMontageAndWaitProxy` "None" "/Game/RadicalMike/Animations/Anim_ZMIKE_UppercutR_Montage.Anim_ZMIKE_UppercutR_Montage" 1.0 "None" true 1.0 0.5
    (:`then`
      (bind _asbp_player (cast `/Game/ProjectAE/Characters/Player/BP_Player` _returnvalue_avataractor))
      (`NiagaraFunctionLibrary.SpawnSystemAttached` "/Game/Fab/VFX/Basic_VFX/Niagara/NS_Basic_11.NS_Basic_11" (`Character.CapsuleComponent` _asbp_player) "None" (0.0 0.0 0.0) (struct) "KeepRelativeOffset"))
    (:`OnCompleted`
      (if (and _bfound_2 _bfound) :!label _label
        (if (>= _returnvalue_4 30.0)
          (bind _returnvalue_5 (`AbilitySystemBlueprintLibrary.AssignTagSetByCallerMagnitude` _returnvalue (struct :`TagName` "Data.Damage") 30.0))
          (`self.K2_ApplyGameplayEffectSpecToOwner` _returnvalue_5)
          (else
            (bind _returnvalue_6 (`AbilitySystemBlueprintLibrary.AssignTagSetByCallerMagnitude` _returnvalue (struct :`TagName` "Data.Damage") _returnvalue_4))
            (`self.K2_ApplyGameplayEffectSpecToOwner` _returnvalue_6)))
        (`self.K2_CommitAbilityCooldown` false)
        (`self.K2_EndAbility`)))
    (:`OnBlendOut`
      (goto _label))
    (:`OnInterrupted`
      (`self.K2_EndAbility` :!label _label_2))
    (:`OnCancelled`
      (goto _label_2))))