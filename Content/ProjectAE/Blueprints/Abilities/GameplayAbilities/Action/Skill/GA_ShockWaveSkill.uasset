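; Player shockwave skill ability that damages and knocks back nearby enemies.
; Plays an uppercut montage, commits cooldown, then waits for the shockwave gameplay event, with a delayed EndAbility as fallback.
; The event triggers a sphere overlap around the player, applying a SetByCaller damage spec and a slow spec to each enemy.
; ApplyEffectForEnemy also stops each enemy's movement and launches it using GetVelocity.
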(event `self.K2_ActivateAbility`
  (bind (_returnvalue_owneractor _returnvalue_avataractor) (break `GameplayAbilityActorInfo` (`self.GetActorInfo`)))
  (`parent.K2_ActivateAbility`)
  (`AbilityTask_PlayMontageAndWait.CreatePlayMontageAndWaitProxy` "ShockWave" "/Game/RadicalMike/Animations/Anim_ZMIKE_UppercutR_Montage.Anim_ZMIKE_UppercutR_Montage" 0.5 "None" true 1.0 0.5
    (:`then`
      (`self.K2_CommitAbilityCooldown` false)
      (`AbilityTask_WaitGameplayEvent.WaitGameplayEvent` (struct :`TagName` "Ability.IsSkill.Shockwave") null
        (:`then`
          (`KismetSystemLibrary.Delay` 4.0)
          (`self.K2_EndAbility` :!label _label))
        (:`EventReceived`
          (bind _asbp_player (cast `/Game/ProjectAE/Characters/Player/BP_Player` _returnvalue_avataractor)
            (:`then`
              (bind _outactors (`KismetSystemLibrary.SphereOverlapActors` (`Actor.K2_GetActorLocation` _asbp_player) 500.0 (`self.Object Types`) null (`|MakeArray` _asbp_player :!type "Actor Object Reference")))
              (bind _output_get (set `self.DamageSpecHandle` (`self.MakeOutgoingGameplayEffectSpec` "/Game/ProjectAE/Blueprints/Abilities/GameplayEffects/Modify/GE_ApplyDamage.GE_ApplyDamage_C")))
              (`AbilitySystemBlueprintLibrary.AssignTagSetByCallerMagnitude` _output_get (struct :`TagName` "Data.Damage") 10.0)
              (set `self.SlowSpecHandle` (`self.MakeOutgoingGameplayEffectSpec` null))
              (for _array_element _outactors
                (bind _asbase_enemy_character (cast `BaseEnemyCharacter` _array_element)
                  (:`then`
                    (`self.ApplyEffectForEnemy` _asbp_player _asbase_enemy_character))
                  (:`CastFailed`
                    (goto _label))))
              (`self.K2_EndAbility`))
            (:`CastFailed`
              (goto _label))))))))

(fn `ApplyEffectForEnemy`
  (params (Player :type "/Game/ProjectAE/Characters/Player/BP_Player Object Reference") (Enemy :type "BaseEnemyCharacter Object Reference"))
  (bind _returnvalue (`BaseCharacter.GetASC` Enemy))
  (bind _returnvalue_2 (`BaseCharacter.GetASC` Player))
  (bind _charactermovement (`Character.CharacterMovement` Enemy))
  (bind (_returnvalue_x _returnvalue_y) (`KismetMathLibrary.BreakVector` (- (`Actor.K2_GetActorLocation` Enemy) (`Actor.K2_GetActorLocation` Player))))
  (`AbilitySystemComponent.BP_ApplyGameplayEffectSpecToTarget` _returnvalue_2 (`self.DamageSpecHandle`) _returnvalue)
  (`AbilitySystemComponent.BP_ApplyGameplayEffectSpecToTarget` _returnvalue_2 (`self.SlowSpecHandle`) _returnvalue)
  (`/Engine/EditorBlueprintResources/StandardMacros.IsValid` _charactermovement
    (:`Is Valid`
      (`MovementComponent.StopMovementImmediately` _charactermovement)
      (`Character.LaunchCharacter` Enemy (+ (* (`KismetMathLibrary.Normal` (`KismetMathLibrary.MakeVector` _returnvalue_x _returnvalue_y)) (`self.KnockbackForce`)) (`KismetMathLibrary.MakeVector` 0.0 0.0 (`self.UpwardForce`))) true true))))