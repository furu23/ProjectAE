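; Gameplay ability that fires one bullet from the player's buster, then ends.
; It finds the pawn through the owning PlayerState, and with ammo left plays the fire montage, spends a round and applies a drained-state effect at zero.
; The bullet spawns at the muzzle socket carrying a SetByCaller damage spec, with a fire trail while overheating.
; Each shot also applies GE_FireInstance and makes pawn noise.
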(event `self.K2_ActivateAbility`
  (bind _ascharacter (`self.GetCharacter`))
  (`self.FireBullet` _ascharacter)
  (`self.K2_EndAbility`))

(fn `GetCharacter`
  (returns (AsCharacter :type "Character Object Reference"))
  (bind _asplayer_state (cast `PlayerState` (`self.GetOwningActorFromActorInfo`)))
  (bind _ascharacter (cast `Character` (`PlayerState.GetPawn` _asplayer_state)))
  (return _ascharacter))