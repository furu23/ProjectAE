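; GA_Fire is a gameplay ability for automatic firing while the fire input is held.
; On activation it calls FireBullet, waits a short delay with a WaitDelay task, and repeats while the owner's ability system component has the Input.Fire tag, otherwise ending the ability.
; FireBullet is currently a placeholder that only prints a debug string.
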(event `self.K2_ActivateAbility`
  (`self.FireLoop`))

(event `FireLoop`
  (`self.FireBullet` :!label _label)
  (`AbilityTask_WaitDelay.WaitDelay` 0.1
    (:`OnFinish`
      (if (`GameplayTagAssetInterface.HasMatchingGameplayTag` (`self.GetAbilitySystemComponentFromActorInfo` self) (struct :`TagName` "Input.Fire"))
        (goto _label)
        (else
          (`self.K2_EndAbility`))))))

(fn `FireBullet`
  (`KismetSystemLibrary.PrintString` "Fire!")
  (return))