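; Gameplay ability that handles the level transition to the lobby, as its name indicates.
; On activation it plays a forward fade message on the first player controller, waits through a short retriggerable delay, then saves through the SaveGame subsystem.
; It then opens the level referenced by the OpenLevel variable and ends the ability.
; An invalid save subsystem only prints a warning, and OpenLevel's RepNotify is empty.
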(event `self.K2_ActivateAbility`
  (message `/Game/ProjectAE/Characters/Player/BPI_UIAnimHandler.ShowFadeAnim` (`GameplayStatics.GetPlayerController` 0) "Forward")
  (`KismetSystemLibrary.RetriggerableDelay` 2.0)
  (`self.DoSaveGame`)
  (`GameplayStatics.OpenLevelBySoftObjectPtr` (`self.OpenLevel`))
  (`self.K2_EndAbility`))

(fn `DoSaveGame`
  (bind _returnvalue (subsystem `SaveGameSubsystem`))
  (`/Engine/EditorBlueprintResources/StandardMacros.IsValid` _returnvalue
    (:`Is Valid`
      (`SaveGameSubsystem.SaveGame` _returnvalue false))
    (:`Is Not Valid`
      (`AEGlobalHelper.PrintString` "Not Valid SaveSys In Transition node" 2.0 (struct :`B` 255 :`G` 255 :`R` 255 :`A` 255) true)))
  (return))

(fn `OnRep_OpenLevel`)