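; GA_LevelTransition is a gameplay ability that moves the game to another level once a required event is completed.
; On activation it checks EventTag against the save game subsystem and ends immediately if that event is not completed.
; Otherwise it plays a fade message on the player controller, waits briefly, calls DoSaveGame and opens the OpenLevel reference.
; DoSaveGame and the OpenLevel rep-notify have empty bodies here.
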(event `self.K2_ActivateAbility`
  (if (`SaveGameSubsystem.IsEventCompleted` (subsystem `SaveGameSubsystem`) (`self.Event Tag`))
    (message `/Game/ProjectAE/Characters/Player/BPI_UIAnimHandler.ShowFadeAnim` (`GameplayStatics.GetPlayerController` 0) "Forward")
    (`KismetSystemLibrary.RetriggerableDelay` 2.0)
    (`self.DoSaveGame`)
    (`GameplayStatics.OpenLevelBySoftObjectPtr` (`self.OpenLevel`))
    (`self.K2_EndAbility`)
    (else
      (`self.K2_EndAbility`))))

(fn `DoSaveGame`)

(fn `OnRep_OpenLevel`)