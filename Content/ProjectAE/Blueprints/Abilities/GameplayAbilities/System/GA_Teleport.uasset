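; GA_Teleport is a gameplay ability that moves the player character to a teleporter's destination.
; On activation it plays a screen fade through the player controller, waits two seconds, then reads the BP_Teleporter source object and teleports the character to its Destination, keeping the current rotation.
; When the ability ends, it reverses the fade and restores normal input mode on the controller.
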(event `self.K2_ActivateAbility`
  (bind _returnvalue (`GameplayStatics.GetPlayerCharacter` 0))
  (message `/Game/ProjectAE/Characters/Player/BPI_UIAnimHandler.ShowFadeAnim` (`GameplayStatics.GetPlayerController` 0) "Forward")
  (`KismetSystemLibrary.RetriggerableDelay` 2.0)
  (bind _asbp_teleporter (cast `/Game/ProjectAE/Blueprints/Interactions/BP_Teleporter` (`self.GetCurrentSourceObject`)))
  (`Actor.K2_TeleportTo` _returnvalue (`SceneComponent.K2_GetComponentLocation` (`/Game/ProjectAE/Blueprints/Interactions/BP_Teleporter.Destination` _asbp_teleporter)) (`Actor.K2_GetActorRotation` _returnvalue))
  (`self.K2_EndAbility`))

(event `self.K2_OnEndAbility`
  (params (bWasCancelled :type Boolean))
  (bind _returnvalue (`GameplayStatics.GetPlayerController` 0))
  (message `/Game/ProjectAE/Characters/Player/BPI_UIAnimHandler.ShowFadeAnim` _returnvalue "Reverse")
  (message `/Game/ProjectAE/Characters/Player/BPI_UIAnimHandler.SetNormalInputMode` _returnvalue))