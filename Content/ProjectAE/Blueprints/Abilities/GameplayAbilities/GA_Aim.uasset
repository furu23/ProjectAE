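; Gameplay ability that puts the player character into an aiming state until the Input.Aim tag is removed.
; Activation reaches the PlayerCharacter through the owning PlayerState's pawn, sets IsAiming, faces it along controller rotation and reduces walk speed.
; Tag removal ends the ability, which clears IsAiming, restores orient-to-movement and adds the speed reduction back onto the current max speed rather than restoring a cached value.
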(event `self.K2_ActivateAbility`
  (`parent.K2_ActivateAbility`)
  (bind _asplayer_state (cast `PlayerState` (`self.GetOwningActorFromActorInfo`)))
  (bind _returnvalue (`PlayerState.GetPawn` _asplayer_state))
  (`/Engine/EditorBlueprintResources/StandardMacros.IsValid` _returnvalue
    (:`Is Valid`
      ;[1 1 1] 반드시 PlayerCharacter의 하위클래스가 Aim Ability의 보유자여야 합니다.
      (bind _asplayer_character (cast `PlayerCharacter` _returnvalue))
      (set `PlayerCharacter.bIsAiming` true _asplayer_character)
      (`self.ApplyAimingState` _asplayer_character)
      (`AbilityTask_WaitGameplayTagRemoved.WaitGameplayTagRemove` (struct :`TagName` "Input.Aim") null true
        (:`Removed`
          (`self.K2_EndAbility`))))))

(event `self.K2_OnEndAbility`
  (params (bWasCancelled :type Boolean))
  (`parent.K2_OnEndAbility` false)
  (bind _asplayer_state (cast `PlayerState` (`self.GetOwningActorFromActorInfo`)))
  (bind _returnvalue (`PlayerState.GetPawn` _asplayer_state))
  (`/Engine/EditorBlueprintResources/StandardMacros.IsValid` _returnvalue
    (:`Is Valid`
      (bind _asplayer_character (cast `PlayerCharacter` _returnvalue))
      (`/Engine/EditorBlueprintResources/StandardMacros.IsValid` _asplayer_character
        (:`Is Valid`
          (set `PlayerCharacter.bIsAiming` false _asplayer_character)
          (`self.RemoveAimingState` _asplayer_character))))))